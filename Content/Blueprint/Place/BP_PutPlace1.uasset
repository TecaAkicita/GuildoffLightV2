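; BP_PutPlace1 is a placement spot where BP_Char hands over a carried item, which triggers a cutscene.
; Overlapping the Sphere while holding an item shows the prompt widget and opens a Gate for the IA_EClick input; leaving hides it and closes the Gate.
; The first accepted press clears HaveItem, sets CanOpen, plays a sound and shows WB_CutScene, followed by WB_Titr after a timed delay.
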(event `self.ReceiveBeginPlay`
  (`self.EnableInput` (`GameplayStatics.GetPlayerController` 0)))

(event `EnhancedInput|/Game/Blueprint/Input/IA_EClick`
  (params (ActionValue :type Boolean) (ElapsedSeconds :type "Float (double-precision)") (TriggeredSeconds :type "Float (double-precision)") (InputAction :type "InputAction Object Reference" :default "/Game/Blueprint/Input/IA_EClick.IA_EClick"))
  (:`Triggered`
    (`/Engine/EditorBlueprintResources/StandardMacros.Gate` true :!label _label
      (:`Exit`
        (`/Engine/EditorBlueprintResources/StandardMacros.DoOnce` false
          (:`Completed`
            (set `/Game/Blueprint/Char/BP_Char.HaveItem?` false (stale `self.Sphere.OnComponentBeginOverlap` _asbp_char))
            (set `/Game/Blueprint/Char/BP_Char.CanOpen?` true (stale `self.Sphere.OnComponentBeginOverlap` _asbp_char))
            (`SceneComponent.SetVisibility` (`self.Widget`) false false)
            (`GameplayStatics.PlaySoundAtLocation` "/Game/SoundEffects/PickUpItem.PickUpItem" (0.0 0.0 0.0) (struct) 1.0 1.0 0.0 null null null null)
            (bind _returnvalue (`|CreateWidget` "/Game/UI_MainMenu/VideoWiget/WB_CutScene.WB_CutScene_C"))
            (`UserWidget.AddToViewport` _returnvalue 0)
            (`KismetSystemLibrary.Delay` 15.0)
            (bind _returnvalue_2 (`|CreateWidget` "/Game/UI_MainMenu/VideoWiget/Titr/WB_Titr.WB_Titr_C"))
            (`UserWidget.AddToViewport` _returnvalue_2 0)))))))

(event `self.Sphere.OnComponentBeginOverlap`
  (params (OverlappedComponent :type "PrimitiveComponent Object Reference") (OtherActor :type "Actor Object Reference") (OtherComp :type "PrimitiveComponent Object Reference") (OtherBodyIndex :type Integer) (bFromSweep :type Boolean) (SweepResult :type "HitResult Structure (by ref)"))
  (bind _asbp_char (cast `/Game/Blueprint/Char/BP_Char` OtherActor))
  (if (`/Game/Blueprint/Char/BP_Char.HaveItem?` _asbp_char)
    (`SceneComponent.SetVisibility` (`self.Widget`) true false)
    (goto _label :!via `Open`)))

(event `self.Sphere.OnComponentEndOverlap`
  (params (OverlappedComponent :type "PrimitiveComponent Object Reference") (OtherActor :type "Actor Object Reference") (OtherComp :type "PrimitiveComponent Object Reference") (OtherBodyIndex :type Integer))
  (cast `/Game/Blueprint/Char/BP_Char` OtherActor)
  (`SceneComponent.SetVisibility` (`self.Widget`) false false)
  (goto _label :!via `Close`))

(fn `UserConstructionScript`)