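; BP_BaseItemPickUpScream is an item pickup that plays a pickup sound and a scream when the player collects it.
; Its sphere overlap with BP_Char shows or hides a widget and opens or closes a gate on the IA_ItemCombo input.
; Input through the open gate sets HaveItem on the character, plays both sounds at world origin rather than the item's location, and destroys the actor.
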(event `self.ReceiveBeginPlay`
  (`self.EnableInput` (`GameplayStatics.GetPlayerController` 0)))

(event `EnhancedInput|/Game/Blueprint/Input/IA_ItemCombo`
  (params (ActionValue :type Boolean) (ElapsedSeconds :type "Float (double-precision)") (TriggeredSeconds :type "Float (double-precision)") (InputAction :type "InputAction Object Reference" :default "/Game/Blueprint/Input/IA_ItemCombo.IA_ItemCombo"))
  (:`Triggered`
    (`/Engine/EditorBlueprintResources/StandardMacros.Gate` true :!label _label
      (:`Exit`
        (set `/Game/Blueprint/Char/BP_Char.HaveItem?` true (stale `self.Sphere.OnComponentBeginOverlap` _asbp_char))
        (`GameplayStatics.PlaySoundAtLocation` "/Game/SoundEffects/PickUpItem.PickUpItem" (0.0 0.0 0.0) (struct) 1.0 1.0 0.0 null null null null)
        (`GameplayStatics.PlaySoundAtLocation` "/Game/SoundEffects/SCREAMINGBIGBROTHER.SCREAMINGBIGBROTHER" (0.0 0.0 0.0) (struct) 1.0 1.0 0.0 null null null null)
        (`self.K2_DestroyActor`)
        (`KismetSystemLibrary.PrintText` "Have item")))))

(event `self.Sphere.OnComponentBeginOverlap`
  (params (OverlappedComponent :type "PrimitiveComponent Object Reference") (OtherActor :type "Actor Object Reference") (OtherComp :type "PrimitiveComponent Object Reference") (OtherBodyIndex :type Integer) (bFromSweep :type Boolean) (SweepResult :type "HitResult Structure (by ref)"))
  (bind _asbp_char (cast `/Game/Blueprint/Char/BP_Char` OtherActor))
  (`SceneComponent.SetVisibility` (`self.Widget`) true false)
  (goto _label :!via `Open`))

(event `self.Sphere.OnComponentEndOverlap`
  (params (OverlappedComponent :type "PrimitiveComponent Object Reference") (OtherActor :type "Actor Object Reference") (OtherComp :type "PrimitiveComponent Object Reference") (OtherBodyIndex :type Integer))
  (cast `/Game/Blueprint/Char/BP_Char` OtherActor)
  (`SceneComponent.SetVisibility` (`self.Widget`) false false)
  (goto _label :!via `Close`))

(fn `UserConstructionScript`)