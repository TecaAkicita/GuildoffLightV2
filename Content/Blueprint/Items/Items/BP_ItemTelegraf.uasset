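; Telegraph item that shows a text message when the player interacts with it.
; Overlap of BP_Char with the Sphere shows a prompt widget and opens a Gate that lets the E key through; leaving hides it and closes the Gate.
; E swaps the prompt for a WBP_TextOnHead widget filled with ContentToShow, then restores the prompt after a three-second delay, without rechecking the overlap.
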(event `self.ReceiveBeginPlay`
  (`self.EnableInput` (`GameplayStatics.GetPlayerController` 0)))

(event `Key|E`
  (params (Key :type "Key Structure"))
  (bind _widget1 (`self.Widget1`))
  (:`Pressed`
    (`/Engine/EditorBlueprintResources/StandardMacros.Gate` true :!label _label
      (:`Exit`
        (`SceneComponent.SetVisibility` (`self.Widget`) false false)
        (bind _output_get (set `self.Widget Promt` (`WidgetComponent.GetUserWidgetObject` (`self.Widget1`))))
        (bind _aswbp_text_on_head (cast `/Game/UI/WBP_TextOnHead` _output_get))
        (set `/Game/UI/WBP_TextOnHead.Content` (`self.Content to Show`) _aswbp_text_on_head)
        (`SceneComponent.SetVisibility` _widget1 true false)
        (`KismetSystemLibrary.Delay` 3.0)
        (`SceneComponent.SetVisibility` _widget1 false false)
        (`SceneComponent.SetVisibility` (`self.Widget`) true false)))))

(event `self.Sphere.OnComponentBeginOverlap`
  (params (OverlappedComponent :type "PrimitiveComponent Object Reference") (OtherActor :type "Actor Object Reference") (OtherComp :type "PrimitiveComponent Object Reference") (OtherBodyIndex :type Integer) (bFromSweep :type Boolean) (SweepResult :type "HitResult Structure (by ref)"))
  (cast `/Game/Blueprint/Char/BP_Char` OtherActor)
  (`SceneComponent.SetVisibility` (`self.Widget`) true false)
  (goto _label :!via `Open`))

(event `self.Sphere.OnComponentEndOverlap`
  (params (OverlappedComponent :type "PrimitiveComponent Object Reference") (OtherActor :type "Actor Object Reference") (OtherComp :type "PrimitiveComponent Object Reference") (OtherBodyIndex :type Integer))
  (cast `/Game/Blueprint/Char/BP_Char` OtherActor)
  (`SceneComponent.SetVisibility` (`self.Widget`) false false)
  (goto _label :!via `Close`))

(fn `UserConstructionScript`)