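; BP_player handles movement input for the player's BP_Char character.
; On BeginPlay it casts player character 0 to BP_Char and stores the reference.
; The MoveForward and MoveRight axes feed AddMovementInput on that character, relative to its camera.
; Forward uses only the camera's yaw, so pitch does not affect the direction, while strafing uses the camera's right vector.
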(event `self.ReceiveBeginPlay`
  (bind _asbp_char (cast `/Game/Blueprint/Char/BP_Char` (`GameplayStatics.GetPlayerCharacter` 0)))
  (set `self.As BP Char` _asbp_char))

(event `InputAxis|MoveForward`
  (params (AxisValue :type "Float (single-precision)"))
  (bind _as_bp_char (`self.As BP Char`))
  (`Pawn.AddMovementInput` _as_bp_char (`KismetMathLibrary.GetForwardVector` (`KismetMathLibrary.MakeRotator` 0.0 0.0 (.yaw (`SceneComponent.K2_GetComponentRotation` (`/Game/Blueprint/Char/BP_Char.Camera` _as_bp_char))))) AxisValue false))

(event `InputAxis|MoveRight`
  (params (AxisValue :type "Float (single-precision)"))
  (bind _as_bp_char (`self.As BP Char`))
  (`Pawn.AddMovementInput` _as_bp_char (`SceneComponent.GetRightVector` (`/Game/Blueprint/Char/BP_Char.Camera` _as_bp_char)) AxisValue false))

(fn `UserConstructionScript`)