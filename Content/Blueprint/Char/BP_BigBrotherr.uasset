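; BP_BigBrotherr is a talking character that shows three timed lines of overhead text when BP_Char enters its Sphere.
; Each line is written into the Govorit widget component's WBP_TextOnHead, shown for four seconds and hidden, with a sound played at world origin.
; Overlap also enables player input on this actor and leaving disables it, though the dialogue sequence continues regardless.
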(event `self.Sphere.OnComponentBeginOverlap`
  (params (OverlappedComponent :type "PrimitiveComponent Object Reference") (OtherActor :type "Actor Object Reference") (OtherComp :type "PrimitiveComponent Object Reference") (OtherBodyIndex :type Integer) (bFromSweep :type Boolean) (SweepResult :type "HitResult Structure (by ref)"))
  (cast `/Game/Blueprint/Char/BP_Char` OtherActor)
  (`self.EnableInput` (`GameplayStatics.GetPlayerController` 0))
  (bind _output_get (set `self.NewVar` (`WidgetComponent.GetUserWidgetObject` (`self.Govorit`))))
  (bind _aswbp_text_on_head (cast `/Game/UI/WBP_TextOnHead` _output_get))
  (set `/Game/UI/WBP_TextOnHead.Content` (`self.ContentToShow`) _aswbp_text_on_head)
  (`SceneComponent.SetVisibility` (`self.Govorit`) true false)
  (`GameplayStatics.PlaySoundAtLocation` "/Game/SoundEffects/GovoritBigBro.GovoritBigBro" (0.0 0.0 0.0) (struct) 1.0 1.0 0.0 null null null null)
  (`KismetSystemLibrary.Delay` 4.0)
  (`SceneComponent.SetVisibility` (`self.Govorit`) false false)
  (set `/Game/UI/WBP_TextOnHead.Content` (`self.ContentToShow_0`) _aswbp_text_on_head)
  (`SceneComponent.SetVisibility` (`self.Govorit`) true false)
  (`GameplayStatics.PlaySoundAtLocation` "/Game/SoundEffects/GovoritBigBro.GovoritBigBro" (0.0 0.0 0.0) (struct) 1.0 1.0 0.0 null null null null)
  (`KismetSystemLibrary.Delay` 4.0)
  (`SceneComponent.SetVisibility` (`self.Govorit`) false false)
  (set `/Game/UI/WBP_TextOnHead.Content` (`self.ContentToShow_1`) _aswbp_text_on_head)
  (`SceneComponent.SetVisibility` (`self.Govorit`) true false)
  (`GameplayStatics.PlaySoundAtLocation` "/Game/SoundEffects/GovoritBigBro.GovoritBigBro" (0.0 0.0 0.0) (struct) 1.0 1.0 0.0 null null null null)
  (`KismetSystemLibrary.Delay` 4.0)
  (`SceneComponent.SetVisibility` (`self.Govorit`) false false))

(event `self.Sphere.OnComponentEndOverlap`
  (params (OverlappedComponent :type "PrimitiveComponent Object Reference") (OtherActor :type "Actor Object Reference") (OtherComp :type "PrimitiveComponent Object Reference") (OtherBodyIndex :type Integer))
  (cast `/Game/Blueprint/Char/BP_Char` OtherActor)
  (`self.DisableInput` (`GameplayStatics.GetPlayerController` 0)))

(fn `UserConstructionScript`)