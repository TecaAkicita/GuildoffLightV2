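; Player character blueprint with a camera that trails the character along a spline and turns to face it.
; BeginPlay adds the IA_Default input mapping and starts a fast looping timer, apparently driving MoveCam.
; MoveCam eases the camera toward the spline point nearest the character and interpolates its rotation toward them, writing a world-space result as relative rotation.
; The IA_ItemCombo input only prints debug text, including HaveItem.
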(event `MoveCam`
  (`self.LookToPerson`)
  (`self.MoveToSpline`))

(event `self.ReceiveBeginPlay`
  (bind _asplayer_controller (cast `PlayerController` (`self.GetController`)))
  (`EnhancedInputSubsystemInterface.AddMappingContext` (pcsubsystem `EnhancedInputLocalPlayerSubsystem` _asplayer_controller) "/Game/Blueprint/Input/IA_Default.IA_Default" 0 (struct))
  (`KismetSystemLibrary.K2_SetTimerDelegate` (`|CreateDelegate` :!event `MoveCam`) 0.01 true))

(event `EnhancedInput|/Game/Blueprint/Input/IA_ItemCombo`
  (params (ActionValue :type Boolean) (ElapsedSeconds :type "Float (double-precision)") (TriggeredSeconds :type "Float (double-precision)") (InputAction :type "InputAction Object Reference" :default "/Game/Blueprint/Input/IA_ItemCombo.IA_ItemCombo"))
  (:`Triggered`
    (`KismetSystemLibrary.PrintText` "Item Combo")
    (`KismetSystemLibrary.PrintText` (`KismetTextLibrary.Conv_BoolToText` (`self.HaveItem?`)))))

(fn `LookToPerson`
  (bind _camera (`self.Camera`))
  (`SceneComponent.K2_SetRelativeRotation` (`self.Camera`) (`KismetMathLibrary.RInterpTo` (`SceneComponent.K2_GetComponentRotation` _camera) (`KismetMathLibrary.Conv_VectorToRotator` (- (`self.K2_GetActorLocation`) (`SceneComponent.K2_GetComponentLocation` _camera))) (`GameplayStatics.GetWorldDeltaSeconds`) 2.0) false false))

(fn `MoveToSpline`
  (locals (NewLocalVar :type "Rotator Structure" :default (struct)))
  (bind _camera (`self.Camera`))
  (`SceneComponent.K2_SetWorldLocation` _camera (`KismetMathLibrary.VInterpTo` (`SceneComponent.K2_GetComponentLocation` _camera) (`SplineComponent.FindLocationClosestToWorldLocation` (`self.Spline`) (`self.K2_GetActorLocation`) "World") (`GameplayStatics.GetWorldDeltaSeconds`) 1.0) false false))

(fn `UserConstructionScript`)