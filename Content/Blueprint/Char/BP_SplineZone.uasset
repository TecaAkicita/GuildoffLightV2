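; BP_SplineZone is a zone that hands its spline to the player character, BP_Char, when that character enters it.
; On BeginPlay it caches the player character and assigns the spline immediately if PlayerIn is already true.
; A Box overlap by any BP_Char sets PlayerIn and writes the spline to the cached character's Spline variable.
; The event graph has no end-overlap handling, so it never clears PlayerIn or the assigned spline.
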(event `self.ReceiveBeginPlay`
  (bind _asbp_char (cast `/Game/Blueprint/Char/BP_Char` (`GameplayStatics.GetPlayerCharacter` 0)))
  (set `self.As BP Char` _asbp_char)
  (if (`self.PlayerIn?`)
    (set `/Game/Blueprint/Char/BP_Char.Spline` (`self.Spline`) (`self.As BP Char`))))

(event `self.Box.OnComponentBeginOverlap`
  (params (OverlappedComponent :type "PrimitiveComponent Object Reference") (OtherActor :type "Actor Object Reference") (OtherComp :type "PrimitiveComponent Object Reference") (OtherBodyIndex :type Integer) (bFromSweep :type Boolean) (SweepResult :type "HitResult Structure (by ref)"))
  (cast `/Game/Blueprint/Char/BP_Char` OtherActor)
  (set `self.PlayerIn?` true)
  (set `/Game/Blueprint/Char/BP_Char.Spline` (`self.Spline`) (`self.As BP Char`)))

(fn `UserConstructionScript`)